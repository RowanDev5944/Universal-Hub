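; BP_Wall is a usable actor in the YouCheated mod that sends the player to another area.
; On BeginPlay it sets its static mesh to a merged text-render mesh.
; When used, it teleports the first player character to a fixed location and rotation, then loads the 10x1000Walk4 level as a streamed instance.
; The overlap and tick events are disabled stubs.
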(event EventBeginPlay
  (|CallParentFunction)
  (Components|StaticMesh|SetStaticMesh (Variables|Default|GetStaticMesh) "/Game/Mods/YouCheated/Models/SM_MERGED_TextRenderActor.SM_MERGED_TextRenderActor"))

(event Collision|EventActorBeginOverlap
  (params (OtherActor :type Actor%20Object%20Reference))
  (|CallParentFunction OtherActor) ; This node is disabled and will not be called.\nDrag off pins to build functionality.
)

(event EventTick
  (params (DeltaSeconds :type Float%20%28single-precision%29))
  (|CallParentFunction DeltaSeconds) ; This node is disabled and will not be called.\nDrag off pins to build functionality.
)

(event EventOnActorUsed
  (params (Character :type Character%20Object%20Reference))
  (Transformation|Teleport (Game|GetPlayerCharacter 0) "0,55700.000000,100.000000" "0, 0, 0")
  (Class|LevelStreamingDynamic|LoadLevelInstancebySoftObjectPtr "/Game/Mods/Z_ExampleLevel_P/Levels/10x1000Walk4.10x1000Walk4" "0, 0, 0" "0, 0, 0"))

(fn ConstructionScript
  (|CallParentFunction))